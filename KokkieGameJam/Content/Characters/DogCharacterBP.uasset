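; Dog character Blueprint that sends the dog toward an obstacle when it is not possessed.
; BeginPlay caches its AI controller, and RefreshAIEvents only calls the parent.
; Each Tick looks up a single ObstacleBP and, within range, sets IsOccupied and calls AIMoveTo with debug prints.
; The unpossessed path never checks IsOccupied, so the move reissues every frame in range, while the possessed path does nothing.
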(event `self.Refresh AI Events`
  (`parent.Refresh AI Events`))

(event `self.ReceiveBeginPlay`
  (`parent.ReceiveBeginPlay`)
  (set `self.AIControllerRef` (`AIBlueprintHelperLibrary.GetAIController` self)))

(event `self.ReceiveTick`
  (params (DeltaSeconds :type "Float (single-precision)"))
  (`parent.ReceiveTick` 0.0)
  ;[1 1 1] Check if near obstalce
  (bind _returnvalue (`GameplayStatics.GetActorOfClass` "/Game/Obstacles/ObstacleBP.ObstacleBP_C"))
  (if (< (`self.GetDistanceTo` self _returnvalue) 400.0)
    (if (`self.IsPossessed`)
      (if (`self.IsOccupied`)
        _)
      (else
        (set `self.IsOccupied` true)
        (`|AIMoveTo` self (0.0 0.0 0.0) _returnvalue
          (:`then`
            (`KismetSystemLibrary.PrintString` "1"))
          (:`OnSuccess`
            (`KismetSystemLibrary.PrintString` "2"))
          (:`OnFail`
            (`KismetSystemLibrary.PrintString` "3")))))))

(fn `UserConstructionScript`
  (`parent.UserConstructionScript`))