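; HumanCharacterBP is a human character Blueprint with an unfinished behavior for chasing the dog.
; Its events and construction script only forward to the parent class or are disabled.
; ChaseDog finds the DogCharacterBP actor and tests whether it is over a set distance away, but the branch does nothing and nothing here calls the function.
; Two debug print nodes are left unreachable.
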(event `self.ReceiveTick`
  (params (DeltaSeconds :type "Float (single-precision)"))
  (`parent.ReceiveTick` DeltaSeconds))

(event `self.ReceivePossessed`
  (params (NewController :type "Controller Object Reference"))
  (`parent.ReceivePossessed` null))

(event `self.ReceiveUnpossessed`
  (params (OldController :type "Controller Object Reference"))
  (`parent.ReceiveUnpossessed` null))

(fn `ChaseDog`
  ;[1 1 1] Chase Dog
  (bind _returnvalue (`GameplayStatics.GetActorOfClass` "/Game/Characters/DogCharacterBP.DogCharacterBP_C"))
  (if (> (`self.GetDistanceTo` self _returnvalue) 100.0)
    _))

(fn `UserConstructionScript`
  (`parent.UserConstructionScript`))