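; Game mode Blueprint that ends play when the level's countdown runs out.
; Each Tick it looks up the TimeActor, casts it to TimeActorBP and checks for zero minutes and -1 seconds.
; On that condition it sets TimeUp, waits briefly through a Delay, then opens the MainMenu level.
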(event `self.ReceiveTick`
  (params (DeltaSeconds :type "Float (single-precision)"))
  (bind _returnvalue (`GameplayStatics.GetActorOfClass` "/Script/KokkieGameJam.TimeActor"))
  (bind _astime_actor_bp (cast `/Game/TimeActorBP` _returnvalue))
  (if (== (`TimeActor.Minutes` _astime_actor_bp) 0)
    (if (== (`TimeActor.Seconds` _astime_actor_bp) -1)
      (set `self.Time Up` true)
      (`KismetSystemLibrary.Delay` 2.0)
      (`GameplayStatics.OpenLevel` "MainMenu"))))

(fn `UserConstructionScript`)