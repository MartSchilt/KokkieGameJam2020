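; Cat obstacle that flags itself as a distraction for the dog character when play begins.
; RunAway shifts the root away from the first DogCharacterBP found, teleporting by a tenth of their horizontal offset per call without sweeping.
; TryRemoveDistraction only prints that the dog stays distracted, and the Tick check on IsCurrentDistraction leads to no action.
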(event `self.ReceiveBeginPlay`
  (`parent.ReceiveBeginPlay`)
  (set `self.IsDistracting` true))

(event `self.ReceiveTick`
  (params (DeltaSeconds :type "Float (single-precision)"))
  (`parent.ReceiveTick` DeltaSeconds)
  (if (`self.IsCurrentDistraction`)
    _))

(event `/Game/Obstacles/DistractingObstacleInterface.TryRemoveDistraction`
  (`KismetSystemLibrary.PrintString` "Not working, The dog seems really distracted"))

(event `RunAway`
  (bind (_returnvalue_x _returnvalue_y) (`KismetMathLibrary.BreakVector` (`self.K2_GetActorLocation` self)))
  (`KismetSystemLibrary.PrintString` "Runaway")
  (bind _outactors (`GameplayStatics.GetAllActorsOfClass` "/Game/Characters/DogCharacterBP.DogCharacterBP_C"))
  (bind (_returnvalue_x_2 _returnvalue_y_2) (`KismetMathLibrary.BreakVector` (`self.K2_GetActorLocation` (`|GetArrayItem` _outactors))))
  (`SceneComponent.K2_AddRelativeLocation` (`self.DefaultSceneRoot`) (/ (* (`KismetMathLibrary.MakeVector` (- _returnvalue_x_2 _returnvalue_x) (- _returnvalue_y_2 _returnvalue_y)) -1.0) 10.0) false true))

(fn `UserConstructionScript`
  (`parent.UserConstructionScript`))