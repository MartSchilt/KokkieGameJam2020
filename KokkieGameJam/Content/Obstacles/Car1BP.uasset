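; Car obstacle Blueprint that travels from a start location to an end location, then teleports back to repeat.
; BeginPlay places it at the start with Z 50 and derives a movement vector by comparing start and end, X first (the +Y case moves diagonally).
; Each Tick, MoveTo applies a swept, speed-scaled offset unless stopped, resetting only when the moving axis exactly equals the endpoint, without using delta time.
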(event `self.ReceiveBeginPlay`
  (bind (_startinglocation_x _startinglocation_y) (`KismetMathLibrary.BreakVector` (`self.StartingLocation`)))
  (bind (_endlocation_x _endlocation_y) (`KismetMathLibrary.BreakVector` (`self.EndLocation`)))
  (bind (_startinglocation_x_2 _startinglocation_y_2) (`KismetMathLibrary.BreakVector` (`self.StartingLocation`)))
  (`parent.ReceiveBeginPlay`)
  (`self.K2_TeleportTo` (`KismetMathLibrary.MakeVector` _startinglocation_x_2 _startinglocation_y_2 50.0))
  (if (> _startinglocation_x _endlocation_x)
    (set `self.Movement` (-1.0 0.0 0.0))
    (elif (< _startinglocation_x _endlocation_x)
      (set `self.Movement` (1.0 0.0 0.0))
      (elif (> _startinglocation_y _endlocation_y)
        (set `self.Movement` (0.0 -1.0 0.0))
        (elif (< _startinglocation_y _endlocation_y)
          (set `self.Movement` (1.0 1.0 0.0))
          (else
            (set `self.Movement` (0.0 0.0 0.0))))))))

(event `self.ReceiveTick`
  (params (DeltaSeconds :type "Float (single-precision)"))
  (`self.MoveTo` (`self.EndLocation`) (`self.StartingLocation`)))

(fn `MoveTo`
  (params (EndPoint :type "Vector Structure") (StartNextPoint :type "Vector Structure"))
  (bind (_endpoint_x _endpoint_y) (`KismetMathLibrary.BreakVector` (`local.EndPoint`)))
  (bind (_movement_x _movement_y) (`KismetMathLibrary.BreakVector` (`self.Movement`)))
  (bind (_returnvalue_x _returnvalue_y) (`KismetMathLibrary.BreakVector` (`SceneComponent.K2_GetComponentLocation` (`self.DefaultSceneRoot`))))
  (if (`self.Stop`)
    _
    (elif (or (and (== _returnvalue_x _endpoint_x) (!= _movement_x 0.0)) (and (== _returnvalue_y _endpoint_y) (!= _movement_y 0.0)))
      (`self.K2_TeleportTo` (`local.StartNextPoint`))
      (else
        (`SceneComponent.K2_AddRelativeLocation` (`self.DefaultSceneRoot`) (* (`self.Movement`) (`self.Speed`)) true false)))))

(fn `UserConstructionScript`)